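; Interactive breaker box that hosts a terminal puzzle and, once solved, powers up linked terminals.
; BeginPlay creates a TerminalBase widget from its pages and log entries, shows it on a widget component and binds puzzle completion.
; Completion plays the lever-pull animation, restores player camera and input, disables the box, then activates BP_Terminal_Interactive actors matching the TerminalToUnlock tag.
; The camera-focus, terminal-boot and panel-opening interaction logic is present but disconnected.
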(event Custom|UnlockTerminal
  (Components|Animation|PlayAnimation (Variables|Default|GetObjectSkeletalMesh) "/Game/TempAssets/Breaker/SM_SafetySwitchAnim_Anim_PullLever_002.SM_SafetySwitchAnim_Anim_PullLever_002" false)
  (Utilities|FlowControl|Delay 1.5)
  (Game|Player|SetViewTargetwithBlend (Game|GetPlayerController 0) (Game|GetPlayerCharacter 0) 1.0 "VTBlend_Linear" 0.0 false)
  (Input|SetInputModeGameOnly (Game|GetPlayerController 0) false)
  (Variables|/Script/Engine.PlayerController|SetbShowMouseCursor (Game|GetPlayerController 0) false)
  (Variables|Default|SetComplete true)
  (Collision|SetCollisionEnabled (Variables|Default|GetObjectMesh) "NoCollision")
  (Rendering|SetVisibility (Variables|Default|GetObjectWidget) false false)
  (bind _outactors (Actor|GetAllActorsOfClasswithTag "/Game/PLATFORM_01_SOLVE/Items/Item_Registry/Terminals/BP_Terminal_Interactive.BP_Terminal_Interactive_C" (Variables|Default|GetTerminal%20To%20Unlock)))
  (for _array_element _outactors
    (Variables|/Game/PLATFORM_01_SOLVE/Items/Item_Registry/Terminals/BP_Terminal_Interactive.BP_Terminal_Interactive_C|SetActive _array_element true)
    (Default|Activate _array_element)))

(event EventBeginPlay
  (|CallParentFunction)
  (bind _returnvalue (UserInterface|CreateWidget "/Game/PLATFORM_01_SOLVE/UI/Terminal/TerminalBase.TerminalBase_C" 0 (Variables|Default|GetTerminal%20PAGES) (Variables|Default|GetTerminal%20Log%20Entries) 0))
  (bind _output_get (Variables|Default|SetTerminal%20Widget _returnvalue))
  (UserInterface|SetWidget (Variables|Default|GetWidget) _output_get)
  (EventDispatchers|BindEventtoPuzzleComplete (delegate Custom|UnlockTerminal)))

(event EventPowerCorrected
  (Development|PrintString "Correct"))

(event EventPointerClick
  (Class|WidgetInteractionComponent|PressPointerKey (Variables|Default|GetWidgetInteraction) "LeftMouseButton"))

(event Input|KeyboardEvents|DebugKeyE
  (params (Key :type Key%20Structure :default "None") (ActionValue :type Input%20Action%20Value%20Structure)))

(fn ConstructionScript
  (|CallParentFunction))