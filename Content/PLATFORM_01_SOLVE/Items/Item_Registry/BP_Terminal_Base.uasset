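; Base interactable terminal item that shows a TerminalBase widget built from its page and log data.
; The widget is created on BeginPlay if the terminal is Active, or when PuzzleCompleted activates it.
; Interacting blends the camera to the terminal, shows the cursor, focuses the widget in Game and UI input and boots it.
; PointerClick forwards left mouse presses through WidgetInteraction.
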(event Custom|Activate
  (if (Variables|Default|GetActive)
    (bind _returnvalue (UserInterface|CreateWidget "/Game/PLATFORM_01_SOLVE/UI/Terminal/TerminalBase.TerminalBase_C" 0 (Variables|Default|GetTerminal%20PAGES) (Variables|Default|GetTerminal%20Log%20Entries) self))
    (bind _output_get (Variables|Default|SetTerminalWidget _returnvalue))
    (UserInterface|SetWidget (Variables|Default|GetTerminal%20Widget) _output_get)))

(event EventBeginPlay
  (|CallParentFunction)
  (CallFunction|Activate))

(event Collision|EventActorBeginOverlap
  (params (OtherActor :type Actor%20Object%20Reference)))

(event EventTick
  (params (DeltaSeconds :type Float%20%28single-precision%29)))

(event EventPointerClick
  (Class|WidgetInteractionComponent|PressPointerKey (Variables|Default|GetWidgetInteraction) "LeftMouseButton"))

(event EventPuzzleCompleted
  (Variables|Default|SetActive true)
  (CallFunction|Activate))

(fn ConstructionScript
  (|CallParentFunction))

(fn InteractwithItem
  (params (Player%20Character :type HNGR%20Char%20Object%20Reference))
  (Variables|Default|SetPlayer%20Character Player%20Character)
  (Game|Player|SetViewTargetwithBlend (Game|GetPlayerController 0) self 0.3 "VTBlend_Linear" 0.0 false)
  (Variables|/Script/Engine.PlayerController|SetbShowMouseCursor (Game|GetPlayerController 0) true)
  (Input|SetInputModeGameandUI (Game|GetPlayerController 0) (UserInterface|GetWidget (Variables|Default|GetTerminal%20Widget)) "DoNotLock" true true)
  (Rendering|SetRenderCustomDepth (Variables|Default|GetObjectMesh) false)
  (Default|BootTerminal (Variables|Default|GetTerminalWidget))
  (return 0))