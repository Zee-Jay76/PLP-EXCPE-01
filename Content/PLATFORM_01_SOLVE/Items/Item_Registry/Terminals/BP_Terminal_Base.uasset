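; Base interactable terminal that shows a TerminalBase screen built from its utility pages and log entries once active.
; Completing a puzzle sets it active and creates the widget, with clicks forwarded through a WidgetInteraction left-mouse press.
; Interacting within the activation radius blends the camera to the terminal and boots it on first use, otherwise it shows a deactivated prompt.
; Un-interacting restores the player camera and removes the widget from its parent.
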(event EventBeginPlay
  (|CallParentFunction))

(event EventPointerClick
  (Class|WidgetInteractionComponent|PressPointerKey (Variables|Default|GetWidgetInteraction) "LeftMouseButton"))

(event EventPuzzleCompleted
  (Variables|Default|SetIs%20Active? true)
  (CallFunction|Activate))

(event EventActivate
  (if (Variables|Default|GetIs%20Active?)
    (bind _returnvalue (UserInterface|CreateWidget "/Game/PLATFORM_01_SOLVE/UI/Terminal/TerminalBase.TerminalBase_C" 0 (Variables|Default|GetUtility%20Pages) (Variables|Default|GetTerminal%20Log%20Entries) self))
    (bind _output_get (Variables|Default|SetTerminalWidget _returnvalue))
    (UserInterface|SetWidget (Variables|Default|GetTerminal%20Widget) _output_get)))

(event EventUn-InteractwithOBJ
  (params (Player%20Ref :type HNGR%20Char%20Object%20Reference))
  (CallFunction|RestorePlayerCameraView)
  (Widget|RemovefromParent (stale EventActivate _returnvalue)))

(fn ConstructionScript
  (|CallParentFunction))

(fn InteractwithItem
  (params (Player%20Character :type HNGR%20Char%20Object%20Reference))
  (if (and (Variables|Default|GetIs%20Active?) (Variables|Default|GetWithin%20Activation%20Radius))
    (CallFunction|BlendCameraViewtoOBJ)
    (if (Variables|Default|GetFirst%20Boot?)
      (Variables|Default|SetFirst%20Boot? false)
      (CallFunction|Activate)
      (Default|BootTerminal (Variables|Default|GetTerminalWidget)))
    (return self)
    (else
      (CallFunction|DialoguePrompt (Variables|Default|GetDeactivatedPrompt)))))