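; Interactive terminal item that shows a screen widget and switches the player into using it.
; On BeginPlay it creates the widget class defined in its TerminalDataAssetInfo and assigns it to its Widget component.
; Interacting blends the player's view to the terminal, shows the mouse cursor and sets UI-only input focused on that screen.
; A PointerClick event forwards a left mouse press through the WidgetInteraction component.
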(event EventBeginPlay
  (|CallParentFunction)
  (bind _returnvalue (UserInterface|CreateWidget (Variables|/Game/PLATFORM_01_SOLVE/Items/Item_Registry/Terminals/DA_BP_Termianl.DA_BP_Termianl_C|GetTerminalScreen (Variables|Default|GetTerminalDataAssetInfo))))
  (UserInterface|SetWidget (Variables|Default|GetWidget) _returnvalue))

(event EventInteractwithItem
  (params (Player%20Character :type HNGR%20Char%20Object%20Reference))
  (Game|Player|SetViewTargetwithBlend (Game|GetPlayerController 0) self 0.3 "VTBlend_Linear" 0.0 false)
  (Variables|/Script/Engine.PlayerController|SetbShowMouseCursor (Game|GetPlayerController 0) true)
  (Input|SetInputModeUIOnly (Game|GetPlayerController 0) (UserInterface|GetWidget (Variables|Default|GetWidget)) "DoNotLock" true))

(event EventPointerClick
  (Class|WidgetInteractionComponent|PressPointerKey (Variables|Default|GetWidgetInteraction) "LeftMouseButton"))

(fn ConstructionScript
  (|CallParentFunction))