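; BP_Breaker_Box is an interactable breaker box that hosts a terminal-widget puzzle and unlocks a linked object when solved.
; BeginPlay creates the terminal widget; interacting blends the camera to the box, enables cursor input, boots the terminal and opens the panel once.
; Completion plays the lever animation, returns view and input to the player, disables further interaction and messages ObjectToUnlock.
; PowerCorrected only prints debug text, and tag-based terminal activation is left disconnected.
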(event Custom|UnlockTerminal)

(event EventBeginPlay
  (|CallParentFunction)
  (bind _returnvalue (UserInterface|CreateWidget "/Game/PLATFORM_01_SOLVE/UI/Terminal/TerminalBase.TerminalBase_C" 0 (Variables|Default|GetTerminal%20PAGES) (Variables|Default|GetTerminal%20Log%20Entries) 0 0))
  (bind _output_get (Variables|Default|SetTerminal%20Widget _returnvalue))
  (UserInterface|SetWidget (Variables|Default|GetWidget) _output_get))

(event EventPowerCorrected
  (Development|PrintString "Correct"))

(event EventPointerClick
  (Class|WidgetInteractionComponent|PressPointerKey (Variables|Default|GetWidgetInteraction) "LeftMouseButton"))

(event EventPuzzleCompleted
  (Components|Animation|PlayAnimation (Variables|Default|GetObjectSkeletalMesh) "/Game/TempAssets/Breaker/SM_SafetySwitchAnim_Anim_PullLever_002.SM_SafetySwitchAnim_Anim_PullLever_002" false)
  (Utilities|FlowControl|Delay 1.5)
  (Game|Player|SetViewTargetwithBlend (Game|GetPlayerController 0) (Game|GetPlayerCharacter 0) 1.0 "VTBlend_Linear" 0.0 false)
  (Input|SetInputModeGameOnly (Game|GetPlayerController 0) false)
  (Variables|/Script/Engine.PlayerController|SetbShowMouseCursor (Game|GetPlayerController 0) false)
  (Variables|Default|SetComplete true)
  (Collision|SetCollisionEnabled (Variables|Default|GetObjectMesh) "NoCollision")
  (Rendering|SetVisibility (Variables|Default|GetObjectWidget) false false)
  (Class|InteractionINTFCE|PuzzleCompleted(Message) (Variables|Default|GetObject%20To%20unlock)))

(fn ConstructionScript
  (|CallParentFunction))

(fn InteractwithItem
  (params (Player%20Character :type HNGR%20Char%20Object%20Reference))
  (bind _objectskeletalmesh (Variables|Default|GetObjectSkeletalMesh))
  (if (not (Variables|Default|GetComplete))
    (Game|Player|SetViewTargetwithBlend (Game|GetPlayerController 0) self 1.0 "VTBlend_Linear" 0.0 false)
    (Variables|/Script/Engine.PlayerController|SetbShowMouseCursor (Game|GetPlayerController 0) true)
    (Input|SetInputModeGameandUI (Game|GetPlayerController 0) (UserInterface|GetWidget (Variables|Default|GetWidget)) "DoNotLock" true true)
    (Rendering|SetRenderCustomDepth (Variables|Default|GetObjectMesh) false)
    (Default|BootTerminal (Variables|Default|GetTerminal%20Widget))
    (Utilities|FlowControl|DoOnce false
      (:Completed
        (Components|Animation|PlayAnimation _objectskeletalmesh "/Game/TempAssets/Breaker/SM_SafetySwitchAnim_Anim_PanelOpen.SM_SafetySwitchAnim_Anim_PanelOpen" false)
        (Collision|SetCollisionEnabled _objectskeletalmesh "NoCollision")
        (Rendering|SetRenderCustomDepth (Variables|Default|GetObjectMesh) false)
        (Class|InteractionINTFCE|PlayOBJWidgetAnimation(Message) (UserInterface|GetUserWidgetObject (Variables|Default|GetObjectWidget)) "Reverse")
        (return 0)))))